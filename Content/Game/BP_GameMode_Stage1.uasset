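; Stage 1 game mode that decides stage clear or failure from the state of the boss and the player.
; At BeginPlay it caches the BP_Boss tagged "Boss", then polls it every Tick, calling StageFailed if the player dies first.
; Boss defeat triggers, once, brief slow motion, camera shake, lethal damage to other non-player characters, and StageClear.
; A Cheat event deals the boss damage equal to its HP.
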(event Custom|Cheat
  (bind _boss (Variables|Default|GetBoss))
  (Game|Damage|ApplyDamage _boss (Variables|/Game/Boss/BP_Boss.BP_Boss_C|GetHP _boss) 0 self))

(event EventBeginPlay
  (|CallParentFunction)
  (|GetBoss))

(event EventTick
  (params (DeltaSeconds :type Float%20%28single-precision%29))
  (bind _boss (Variables|Default|GetBoss)
    (:then
      (if (Utilities|Enum|Equal(Enum) (Variables|/Game/Boss/BP_Boss.BP_Boss_C|GetStateType _boss) "NewEnumerator4")
        ;[1 1 1] 스테이지 클리어
        (Utilities|FlowControl|Sequence
          (:then_0
            (Utilities|FlowControl|DoOnce false
              (:Completed
                (Utilities|FlowControl|Sequence
                  (:then_0
                    (Utilities|Time|SetGlobalTimeDilation 0.25)
                    (Class|PlayerCameraManager|PlayCameraShake (Game|GetPlayerCameraManager 0) "/Game/Game/Shake_BossDead.Shake_BossDead_C" 1.0 "CameraLocal" "0, 0, 0")
                    (Utilities|FlowControl|Delay 0.15)
                    (Utilities|Time|SetGlobalTimeDilation 1.0))
                  (:then_1
                    (bind _outactors (Actor|GetAllActorsOfClass "/Script/Engine.Character"))
                    (for _array_element _outactors
                      (Utilities|Casting|CastToBP_Player _array_element
                        (:CastFailed
                          (if (!= _array_element (Variables|Default|GetBoss))
                            (Game|Damage|ApplyDamage _array_element 9999.0 0 self))))))
                  (:then_2
                    (CallFunction|StageClear)))))))
        (else
          (bind _asbp_player (Utilities|Casting|CastToBP_Player (Game|GetPlayerCharacter 0)))
          (if (Variables|/Game/Player/BP_Player.BP_Player_C|GetbDead _asbp_player)
            (CallFunction|StageFailed)))))
    (:else)))

(fn ConstructionScript)