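; BP_GameMode_Stage2 is the game mode for Stage 2, handling stage completion and a cheat teleport.
; BeginPlay runs the parent logic, then caches the first BP_Goal and the first TargetPoint found in the level.
; Tick polls the goal's Clear flag and, once set, disables player input and calls StageClear a single time.
; The Cheat event moves the player character to the cached TargetPoint.
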(event Custom|Cheat
  (Transformation|SetActorLocation (Game|GetPlayerCharacter 0) (Transformation|GetActorLocation (Variables|Default|GetTarget)) false false))

(event EventBeginPlay
  (|CallParentFunction)
  (bind _outactors (Actor|GetAllActorsOfClass "/Game/BluePrint/BP_Goal.BP_Goal_C"))
  (Variables|Default|SetGoal (Utilities|Array|Get(acopy) _outactors))
  (bind _outactors_2 (Actor|GetAllActorsOfClass "/Script/Engine.TargetPoint"))
  (Variables|Default|SetTarget (Utilities|Array|Get(acopy) _outactors_2)))

(event EventTick
  (params (DeltaSeconds :type Float%20%28single-precision%29))
  (if (Variables|/Game/BluePrint/BP_Goal.BP_Goal_C|GetbClear (Variables|Default|GetGoal))
    (Utilities|FlowControl|DoOnce false
      (:Completed
        (Input|DisableInput (Game|GetPlayerCharacter 0) (Game|GetPlayerController 0))
        (CallFunction|StageClear)))))

(fn ConstructionScript)