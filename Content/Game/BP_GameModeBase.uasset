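; Game mode base for stage levels that handles stage clear, failure and the related UI.
; On BeginPlay it creates hidden clear, pause and game-over widgets and parses the stage number from the level name into the game instance.
; Clearing raises the saved highest cleared stage, saves, then shows the clear widget and cursor after a delay.
; Failing shows game over with UI input; a Cheat event only prints a message.
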(event Custom|Cheat
  (Development|PrintString "치트 활성화"))

(event Custom|StageClear
  (bind _returnvalue (Game|GetPlayerController 0))
  (bind _asbp_game_instance (CallFunction|GetMyGameInstance))
  (bind _currentstage (Variables|/Game/Game/BP_GameInstance.BP_GameInstance_C|GetCurrentStage _asbp_game_instance))
  (if (> _currentstage (Variables|/Game/Game/BP_GameInstance.BP_GameInstance_C|GetClearStage _asbp_game_instance))
    (Variables|/Game/Game/BP_GameInstance.BP_GameInstance_C|SetClearStage _asbp_game_instance _currentstage))
  (Default|Save (CallFunction|GetMyGameInstance))
  (Utilities|FlowControl|Delay 2.0)
  (Widget|SetVisibility (Variables|Default|GetStageClearWidget) "Visible")
  (Variables|/Script/Engine.PlayerController|SetbShowMouseCursor _returnvalue true)
  (Input|SetInputModeGameandUI _returnvalue 0 "DoNotLock" true))

(event Custom|StageFailed
  (Widget|SetVisibility (Variables|Default|GetOverWidget) "Visible")
  (CallFunction|InputModetoUI))

(event EventBeginPlay
  (CallFunction|InputModetoGame)
  (|CreateStageClearWIdget)
  (|CreatePauseWidget)
  (|GameOverWIdget)
  (|SetCurrentStage))

(fn ConstructionScript)