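; Player character Blueprint for a sword-and-shield fighter with sideways movement, jumping and a montage attack, viewed through its own camera.
; An Attacking flag gates movement, jumps and new attacks; forward movement logic is left unwired.
; OnCollision/OffCollision toggle the sword collider, whose overlaps apply Atk damage to other actors.
; Incoming damage lowers HP, briefly flashes red through a dynamic material, and at zero plays death and disables input.
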(event OnComponentBeginOverlap(SwordCollision)
  (params (OverlappedComponent :type Primitive%20Component%20Object%20Reference) (OtherActor :type Actor%20Object%20Reference) (OtherComp :type Primitive%20Component%20Object%20Reference) (OtherBodyIndex :type Integer) (bFromSweep :type Boolean) (SweepResult :type Hit%20Result%20Structure%20%28by%20ref%29))
  ;[1 1 1] 데미지 입히기
  (if (!= OtherActor self)
    (Game|Damage|ApplyDamage OtherActor (Variables|Default|GetAtk) 0 self)))

(event Custom|OnCollision
  ;[1 1 1] 무기 충돌체 끄고/켜기
  (Collision|SetCollisionEnabled (Variables|Default|GetSwordCollision) "QueryAndPhysics"))

(event Custom|OffCollision
  ;[1 1 1] 무기 충돌체 끄고/켜기
  (Collision|SetCollisionEnabled (Variables|Default|GetSwordCollision) "NoCollision"))

(event Custom|DamageEffect
  (Rendering|Material|SetVectorParameterValue (Variables|Default|GetDynamicMaterial) "HitColor" "(R=1.000000,G=0.000000,B=0.000000,A=1.000000)" :!class /Script/Engine.MaterialInstanceDynamic)
  (Utilities|FlowControl|Delay 0.1)
  (Rendering|Material|SetVectorParameterValue (Variables|Default|GetDynamicMaterial) "HitColor" "(R=0.000000,G=0.000000,B=0.000000,A=1.000000)" :!class /Script/Engine.MaterialInstanceDynamic))

(event Game|Damage|EventAnyDamage
  (params (Damage :type Float%20%28single-precision%29) (DamageType :type Damage%20Type%20Object%20Reference) (InstigatedBy :type Controller%20Object%20Reference) (DamageCauser :type Actor%20Object%20Reference))
  (Utilities|FlowControl|Sequence
    (:then_0
      (bind _output_get (Variables|Default|SetHP (- (Variables|Default|GetHP) Damage)))
      (if (<= _output_get 0.0)
        (Animation|PlayAnimMontage "/Game/Mixamo/Paladin/Animations/sword_and_shield_death__2__Montage.sword_and_shield_death__2__Montage" 1.0 "None")
        (Variables|Default|SetbDead true)
        (Input|DisableInput 0)))
    (:then_1
      (CallFunction|DamageEffect))))

(event EventBeginPlay
  ;[1 1 1] 메인 카메라 세팅
  (Game|Player|SetViewTargetwithBlend (Game|GetPlayerController 0) (Variables|Default|GetMainCamera) 0.0 "VTBlend_Linear" 0.0 false)
  ;[1 1 1] 다이나믹 머티리얼 생성
  (bind _returnvalue (Rendering|Material|CreateDynamicMaterialInstance "/Game/Mixamo/Paladin/Mesh/Paladin_MAT_Inst.Paladin_MAT_Inst" "None" :!class /Script/Engine.KismetMaterialLibrary))
  (bind _output_get (Variables|Default|SetDynamicMaterial _returnvalue))
  (Rendering|Material|SetMaterial (Variables|Character|GetMesh) 0 _output_get))

(event Input|AxisEvents|InputAxisMoveForward
  (params (AxisValue :type Float%20%28single-precision%29))
  ;[1 1 1] 이동
)

(event Input|AxisEvents|InputAxisMoveRight
  (params (AxisValue :type Float%20%28single-precision%29))
  ;[1 1 1] 이동
  (if (not (Variables|Default|GetbAttacking))
    (Pawn|Input|AddMovementInput "0,1.000000, 0" AxisValue false)))

(event Input|MouseEvents|LeftMouseButton
  (params (Key :type Key%20Structure :default "None"))
  ;[1 1 1] 공격
  (:Pressed
    (if (not (Variables|Default|GetbAttacking))
      (Variables|Default|SetbAttacking true)
      (Animation|PlayAnimMontage "/Game/Mixamo/Paladin/Animations/sword_and_shield_slash_Montage.sword_and_shield_slash_Montage" 1.2 "None"))))

(event Input|KeyboardEvents|SpaceBar
  (params (Key :type Key%20Structure :default "None"))
  ;[1 1 1] 점프
  (:Pressed
    (if (not (Variables|Default|GetbAttacking))
      (Character|Jump)))
  (:Released
    (Character|StopJumping)))

(fn ConstructionScript)