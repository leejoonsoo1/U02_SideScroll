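; Floor7_Blueprint is a floor actor that slides 500 units along negative Y once play begins.
; BeginPlay takes the static mesh component's world location as the start point and derives the end point from it.
; A timeline then drives a vector lerp between the two, setting the actor's location on each update without sweep or teleport.
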(event EventBeginPlay
  (Variables|Default|SetStart (Transformation|GetWorldLocation (Variables|Debug|GetStaticMeshComponent)))
  (Variables|Default|SetEnd (- (Variables|Default|GetStart) "0,500.000000, 0"))
  (bind _새_트랙_0 (Timeline|타임라인_0 Play)
    (:Update
      (Transformation|SetActorLocation (Math|Vector|Lerp(Vector) (Variables|Default|GetStart) (Variables|Default|GetEnd) _새_트랙_0) false false))))

(fn ConstructionScript)