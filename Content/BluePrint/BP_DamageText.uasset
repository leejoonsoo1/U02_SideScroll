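; BP_DamageText is a world-space floating damage number actor that shows a damage value through a TextRender component.
; SetDamageText formats the damage amount into the text.
; On BeginPlay a timeline offsets the actor vertically from its spawn location and drives its uniform scale, then destroys the actor when it finishes.
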(event EventBeginPlay
  (Variables|Default|SetStart (Transformation|GetActorLocation))
  (bind _out (Timeline|Timeline Play)
    (:Update
      (Transformation|SetActorLocation (+ (Variables|Default|GetStart) (Math|Vector|MakeVector 0.0 0.0 (.X (Math|Vector|BreakVector _out)))) false false)
      (Transformation|SetActorScale3D (Math|Conversions|ToVector(Float) (.Y (Math|Vector|BreakVector _out)))))
    (:Finished
      (Actor|DestroyActor))))

(fn ConstructionScript)

(fn SetDamageText
  (params (Damage :type Float%20%28single-precision%29))
  (Rendering|Components|TextRender|SetText (Variables|Default|GetTextRender) (Utilities|Text|ToText(Float) Damage "HalfToEven")))