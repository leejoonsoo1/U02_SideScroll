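; BP_Trap_2 is a moving trap actor that damages the player character on overlap.
; On BeginPlay, a timeline lerps the actor from its static mesh location to a point a short distance below.
; Overlapping actors of the player character's class receive fixed damage.
; A separate TakeDamage function applies Atk damage to every entry in HittedCharacters, but neither event here calls it.
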(event Collision|EventActorBeginOverlap
  (params (OtherActor :type Actor%20Object%20Reference))
  (if (== (Utilities|GetClass OtherActor) (Utilities|GetClass (Game|GetPlayerCharacter 0)))
    (Game|Damage|ApplyDamage OtherActor 1e+01 0 0)))

(event EventBeginPlay
  (Variables|Default|SetStart (Transformation|GetSocketLocation (Variables|Debug|GetStaticMeshComponent) "None"))
  (Variables|Default|SetEnd (+ (Variables|Default|GetStart) "0, 0,-70.000000"))
  (bind _새_트랙_0 (Timeline|타임라인_0 Play)
    (:Update
      (Transformation|SetActorLocation (Math|Vector|Lerp(Vector) (Variables|Default|GetStart) (Variables|Default|GetEnd) _새_트랙_0) false false))))

(fn ConstructionScript)

(fn TakeDamage
  (if (not (< (Utilities|Array|Length (Variables|Default|GetHittedCharacters)) 1))
    (for _array_element (Variables|Default|GetHittedCharacters)
      (Game|Damage|ApplyDamage _array_element (Variables|Default|GetAtk) 0 self))))