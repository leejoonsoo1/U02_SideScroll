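; Melee enemy that chases and attacks the player, measuring distance and direction only along the Y axis.
; Tick drives Idle, Approach and Attack states while the player lives; attack-end and hit events call NextBehavior to re-attack or return to Idle.
; Separate events toggle the weapon collision, whose overlaps damage the player.
; Taking damage causes knockback or death, plus a sound and red flash through a dynamic material.
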(event OnComponentBeginOverlap(WeaponCollision)
  (params (OverlappedComponent :type Primitive%20Component%20Object%20Reference) (OtherActor :type Actor%20Object%20Reference) (OtherComp :type Primitive%20Component%20Object%20Reference) (OtherBodyIndex :type Integer) (bFromSweep :type Boolean) (SweepResult :type Hit%20Result%20Structure%20%28by%20ref%29))
  ;[1 1 1] 무기에 충돌된 엑터에게 데미지 주기
  (if (CallFunction|IsBodyTagValid OtherComp)
    (if (!= OtherActor self)
      (bind _asbp_player (Utilities|Casting|CastToBP_Player OtherActor))
      (Game|Damage|ApplyDamage _asbp_player (Variables|Default|GetAtk) 0 self))))

(event Custom|HitEffect
  ;[1 1 1] 피격 이펙트
  (Audio|PlaySoundatLocation "/Game/Sounds/Hit.Hit" (Transformation|GetActorLocation) "0, 0, 0" 1.0 1.0 0.0 0 0 0)
  (Rendering|Material|SetVectorParameterValue (Variables|Default|GetDynamicMaterial) "HitColor" "(R=1.000000,G=0.000000,B=0.000000,A=1.000000)" :!class /Script/Engine.MaterialInstanceDynamic)
  (Utilities|FlowControl|Delay 0.2)
  (Rendering|Material|SetVectorParameterValue (Variables|Default|GetDynamicMaterial) "HitColor" "(R=0.000000,G=0.000000,B=0.000000,A=1.000000)" :!class /Script/Engine.MaterialInstanceDynamic))

(event Custom|EndAttack
  ;[1 1 1] 공격종료 - 거리가 멀어지면 쫓아가서 재공격
  (CallFunction|NextBehavior))

(event Custom|OnCollision
  ;[1 1 1] 무기 충돌체 끄고/켜기
  (Collision|SetCollisionEnabled (Variables|Default|GetWeaponCollision) "QueryAndPhysics"))

(event Custom|OffCollision
  ;[1 1 1] 무기 충돌체 끄고/켜기
  (Collision|SetCollisionEnabled (Variables|Default|GetWeaponCollision) "NoCollision"))

(event Custom|Hitted
  ;[1 1 1] 피격 시
  (CallFunction|NextBehavior))

(event Custom|NextBehavior
  ;[1 1 1] 공격 끝나면 다음 동작
  (if (not (CallFunction|IsPlayerDead))
    (Variables|Default|SetBeAttacking false)
    (if (> (Variables|Default|GetDistanceToPlayer) (Variables|Default|GetAttackRange))
      (Variables|Default|SetStateType "NewEnumerator0")
      (else
        (Transformation|SetActorRotation (Math|Conversions|RotationFromXVector (Variables|Default|GetDirectionToPlayer)))
        (Animation|PlayAnimMontage "/Game/Mixamo/Goblin/Animations/Standing_Melee_Attack_Downward_Montage.Standing_Melee_Attack_Downward_Montage" 1.25 "None")
        (Variables|Default|SetBeAttacking true)))))

(event EventBeginPlay
  ;[1 1 1] 다이나믹 머티리얼 세팅 (런타임 상황에서도 머티리얼의 값을 변경 가능한 코드)
  (bind _returnvalue (Rendering|Material|CreateDynamicMaterialInstance "/Game/Mixamo/Goblin/Mesh/phong1_Inst.phong1_Inst" "None" :!class /Script/Engine.KismetMaterialLibrary))
  (bind _output_get (Variables|Default|SetDynamicMaterial _returnvalue))
  (Rendering|Material|SetMaterial (Variables|Character|GetMesh) 1 _output_get)
  (Collision|SetCollisionEnabled (Variables|Default|GetWeaponCollision) "NoCollision"))

(event EventTick
  (params (DeltaSeconds :type Float%20%28single-precision%29))
  ;[1 1 1] 틱 - 상태 배경
  (if (not (CallFunction|IsPlayerDead))
    (|CollectPlayerData)
    (switch Utilities|FlowControl|Switch|SwitchonEStateType (Variables|Default|GetStateType)
      (:NewEnumerator0
        (if (<= (Variables|Default|GetDistanceToPlayer) 5e+02)
          (Variables|Default|SetStateType "NewEnumerator1")))
      (:NewEnumerator1
        (if (<= (Variables|Default|GetDistanceToPlayer) 1.6e+02)
          (Variables|Default|SetStateType "NewEnumerator2")
          (Animation|PlayAnimMontage "/Game/Mixamo/Goblin/Animations/Standing_Melee_Attack_Downward_Montage.Standing_Melee_Attack_Downward_Montage" 1.25 "None")
          (Variables|Default|SetBeAttacking true)
          (else
            (Pawn|Input|AddMovementInput (Variables|Default|GetDirectionToPlayer) 1.0 false))))
      (:NewEnumerator2
        (if (not (Variables|Default|GetBeAttacking))
          (if (> (Variables|Default|GetDistanceToPlayer) 1.6e+02)
            (Variables|Default|SetStateType "NewEnumerator1")))))))

(event Game|Damage|EventAnyDamage
  (params (Damage :type Float%20%28single-precision%29) (DamageType :type Damage%20Type%20Object%20Reference) (InstigatedBy :type Controller%20Object%20Reference) (DamageCauser :type Actor%20Object%20Reference))
  ;[1 1 1] 피격 시
  (Collision|SetCollisionEnabled (Variables|Default|GetWeaponCollision) "NoCollision")
  (Variables|Default|SetBeAttacking false)
  (if (Utilities|Enum|NotEqual(Enum) (Variables|Default|GetStateType) "NewEnumerator4")
    (Utilities|FlowControl|Sequence
      (:then_0
        (bind _output_get (Variables|Default|SetHP (- (Variables|Default|GetHP) Damage)))
        (if (<= _output_get 0.0)
          (Variables|Default|SetStateType "NewEnumerator4")
          (Animation|PlayAnimMontage "/Game/Mixamo/Goblin/Animations/Standing_Death_Left_02_Montage.Standing_Death_Left_02_Montage" 1.0 "None")
          (else
            (Character|LaunchCharacter (* (Variables|Default|GetDirectionToPlayer) -500) false false)
            (Variables|Default|SetStateType "NewEnumerator6")
            (Animation|PlayAnimMontage "/Game/Mixamo/Goblin/Animations/Stomach_Hit_Montage.Stomach_Hit_Montage" 1.0 "None"))))
      (:then_1
        (CallFunction|HitEffect)))))

(fn ConstructionScript)

(fn IsPlayerDead
  (bind _asbp_player (Utilities|Casting|CastToBP_Player (Game|GetPlayerCharacter 0)))
  (return (Variables|/Game/Player/BP_Player.BP_Player_C|GetbDead _asbp_player)))